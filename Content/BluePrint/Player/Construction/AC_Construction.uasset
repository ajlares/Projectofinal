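; Player construction component that lets the third-person character place, rotate and destroy buildables.
; BeginPlay loads buildables from a data table, and the mouse wheel selects among them.
; In build mode, a per-tick camera trace moves a ghost mesh, created through a resettable DoOnce, and placing spawns the Blueprint at that transform.
; Switching or exiting clears the preview, while a separate trace destroys "Buildable"-tagged actors even outside build mode.
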(event Custom|Preview%20Look
  (bind _returnvalue (Game|GetPlayerCameraManager 0))
  (bind _returnvalue_2 (Camera|GetCameraLocation _returnvalue))
  ;[0.15 0.15 0.15 0.5] Dibujamos el rayo para la posición de la construcción
  (bind (_outhit _returnvalue_3) (Collision|LineTraceByChannel _returnvalue_2 (+ _returnvalue_2 (* (Math|Vector|GetForwardVector (Camera|GetCameraRotation _returnvalue)) (Variables|Default|GetRayDistance))) "TraceTypeQuery1" false 0 "None"))
  (if _returnvalue_3 ; Si el rayo choca con algo
    (Utilities|FlowControl|Sequence
      (:then_0
        (Utilities|FlowControl|DoOnce false
          (:Completed
            ;[0.15 0.15 0.15 0.5] Le agregamos un componente Static mesh al player
            (bind _returnvalue_4 (Game|AddComponentbyClass (Variables|Default|GetPlayerBP) "/Script/Engine.StaticMeshComponent" false (Variables|Default|GetBuildPreviewTransform)))
            ;[0.15 0.15 0.15 0.5] Agregamos mesh
            (bind _output_get (Variables|Default|SetPreviewMesh _returnvalue_4)) ; el mesh agregado a platyer lo hacemos variable
            (Components|StaticMesh|SetStaticMesh _output_get (.Mesh (Utilities|Struct|BreakS_ConstructionElements (Utilities|Array|Get(acopy) (Variables|Default|GetDT_Buildables) (Variables|Default|GetBuildableIndex))))) ; Aqui se asigna el mesh del preview
            (Rendering|Material|SetMaterial (Variables|Default|GetPreviewMesh) 0 "/Game/Materials/MAT_BuildingPreview.MAT_BuildingPreview")
            (Collision|SetCollisionEnabled (Variables|Default|GetPreviewMesh) "NoCollision"))))
      (:then_1
        ;[0.15 0.15 0.15 0.5] Mostramos el preview donde choca el rayo
        (bind _output_get_2 (Variables|Default|SetBuildPreviewTransform (Math|Transform|MakeTransform (.Location (Collision|BreakHitResult _outhit)) (Variables|Default|GetBuildPreviewRotation) "1.000000,1.000000,1.000000"))) ; La ubicación en la que choque el rayo la guardamos en una variable
        (Transformation|SetWorldTransform (Variables|Default|GetPreviewMesh) _output_get_2 false false)))))

(event Custom|Reset%20Build%20Mode
  (Utilities|FlowControl|DoOnce false) ; enters at Reset
)

(event Custom|Stop%20Build%20Mode
  ;[0.15 0.15 0.15 0.5] Entrar y salir de preview mode
  ;;[0.15 0.15 0.15 0.5] Al salir de la construcción reseteamos el preview
  (Variables|Default|SetInBuildMode false)
  (bind _previewmesh (Variables|Default|GetPreviewMesh)
    (:then
      (Components|StaticMesh|SetStaticMesh _previewmesh 0)
      (Variables|Default|SetPreviewMesh 0)
      (CallFunction|ResetBuildMode))
    (:else)))

(event Input|EnhancedActionEvents|EnhancedInputActionIA_Build
  (params (ActionValue :type Boolean) (ElapsedSeconds :type Float%20%28double-precision%29) (TriggeredSeconds :type Float%20%28double-precision%29) (InputAction :type Input%20Action%20Object%20Reference :default "/Game/ThirdPerson/Input/Actions/Building/IA_Build.IA_Build"))
  ;[0.15 0.15 0.15 0.5] Entrar y salir de preview mode
  (:Started
    (if (not (Variables|Default|GetInBuildMode))
      (Variables|Default|SetInBuildMode true)
      (else
        ;;[0.15 0.15 0.15 0.5] Al salir de la construcción reseteamos el preview
        (Variables|Default|SetInBuildMode false)
        (bind _previewmesh (Variables|Default|GetPreviewMesh)
          (:then
            (Components|StaticMesh|SetStaticMesh _previewmesh 0)
            (Variables|Default|SetPreviewMesh 0)
            (CallFunction|ResetBuildMode))
          (:else))))))

(event Input|EnhancedActionEvents|EnhancedInputActionIA_PlaceBuild
  (params (ActionValue :type Boolean) (ElapsedSeconds :type Float%20%28double-precision%29) (TriggeredSeconds :type Float%20%28double-precision%29) (InputAction :type Input%20Action%20Object%20Reference :default "/Game/ThirdPerson/Input/Actions/Building/IA_PlaceBuild.IA_PlaceBuild"))
  ;[0.15 0.15 0.15 0.5] Colocamos al objeto donde está el preview
  (:Started
    (if (Variables|Default|GetInBuildMode)
      (Game|SpawnActorfromClass (.Blueprint (Utilities|Struct|BreakS_ConstructionElements (Utilities|Array|Get(acopy) (Variables|Default|GetDT_Buildables) (Variables|Default|GetBuildableIndex)))) (Variables|Default|GetBuildPreviewTransform) "AlwaysSpawn" "MultiplyWithRoot" 0 0)
      (CallFunction|StopBuildMode))))

(event Input|EnhancedActionEvents|EnhancedInputActionIA_RotateBuildRight
  (params (ActionValue :type Boolean) (ElapsedSeconds :type Float%20%28double-precision%29) (TriggeredSeconds :type Float%20%28double-precision%29) (InputAction :type Input%20Action%20Object%20Reference :default "/Game/ThirdPerson/Input/Actions/Building/IA_RotateBuildRight.IA_RotateBuildRight"))
  ;[0.15 0.15 0.15 0.5] Hacemos rotar al objeto
  (:Ongoing
    (Variables|Default|SetBuildPreviewRotation (Math|Rotator|CombineRotators (.rotation (Variables|Default|GetBuildPreviewTransform)) "0.000000,1.000000,0.000000"))))

(event Input|EnhancedActionEvents|EnhancedInputActionIA_RotateBuildLeft
  (params (ActionValue :type Boolean) (ElapsedSeconds :type Float%20%28double-precision%29) (TriggeredSeconds :type Float%20%28double-precision%29) (InputAction :type Input%20Action%20Object%20Reference :default "/Game/ThirdPerson/Input/Actions/Building/IA_RotateBuildLeft.IA_RotateBuildLeft"))
  ;[0.15 0.15 0.15 0.5] Hacemos rotar al objeto
  (Variables|Default|SetBuildPreviewRotation (Math|Rotator|CombineRotators (.rotation (Variables|Default|GetBuildPreviewTransform)) "0.000000,-1.000000,0.000000")))

(event Input|EnhancedActionEvents|EnhancedInputActionIA_DestroyBuild
  (params (ActionValue :type Boolean) (ElapsedSeconds :type Float%20%28double-precision%29) (TriggeredSeconds :type Float%20%28double-precision%29) (InputAction :type Input%20Action%20Object%20Reference :default "/Game/ThirdPerson/Input/Actions/Building/IA_DestroyBuild.IA_DestroyBuild"))
  (bind _returnvalue (Game|GetPlayerCameraManager 0))
  (bind _returnvalue_2 (Camera|GetCameraLocation _returnvalue))
  (bind (_outhit _returnvalue_3) (Collision|LineTraceByChannel _returnvalue_2 (+ _returnvalue_2 (* (Math|Vector|GetForwardVector (Camera|GetCameraRotation _returnvalue)) (Variables|Default|GetRayDistance))) "TraceTypeQuery1" false 0 "None"))
  (if _returnvalue_3 ; Si el rayo choca con algo
    (if (Actor|ActorHasTag (.HitActor (Collision|BreakHitResult _outhit)) "Buildable")
      (Actor|DestroyActor (.HitActor (Collision|BreakHitResult _outhit))))))

(event EventBeginPlay
  ;[0.15 0.15 0.15 0.5] Conseguir referencia a BP player
  (bind _asbp_third_person_character (Utilities|Casting|CastToBP_ThirdPersonCharacter (Components|GetOwner)))
  (Variables|Default|SetPlayerBP _asbp_third_person_character)
  ;[0.15 0.15 0.15 0.5] Conseguimos la DT con todos los construibles. Asignamos las rows a una variable
  (bind _outrownames (DataTable|GetDataTableRowNames "/Game/BluePrint/Player/Construction/DT_COnstructionElements.DT_COnstructionElements"))
  (for _array_element _outrownames
    (bind _returnvalue (Utilities|GetDataTableRow "/Game/BluePrint/Player/Construction/DT_COnstructionElements.DT_COnstructionElements" _array_element)
      (:then
        (Utilities|Array|Add (Variables|Default|GetDT_Buildables) _returnvalue)))))

(event EventTick
  (params (DeltaSeconds :type Float%20%28single-precision%29))
  ;[0.15 0.15 0.15 0.5] Ejecutamos el build mode
  (if (Variables|Default|GetInBuildMode)
    (CallFunction|PreviewLook)))

(event Input|MouseEvents|MouseWheelDown
  (params (Key :type Key%20Structure :default "None"))
  ;[0.15 0.15 0.15 0.5] Recorrer lista de elementos construibles
  (:Pressed
    (Variables|Default|SetBuildableIndex (Math|Integer|Clamp(Integer) (+ (Variables|Default|GetBuildableIndex) 1) 0 (- (Utilities|Array|Length (Variables|Default|GetDT_Buildables)) 1)))
    ;[0.15 0.15 0.15 0.5] Hacemos que se actualice el mesh en el preview mode
    (bind _previewmesh (Variables|Default|GetPreviewMesh)
      (:then
        (Components|StaticMesh|SetStaticMesh _previewmesh 0)
        (Variables|Default|SetPreviewMesh 0)
        (CallFunction|ResetBuildMode))
      (:else))))

(event Input|MouseEvents|MouseWheelUp
  (params (Key :type Key%20Structure :default "None"))
  ;[0.15 0.15 0.15 0.5] Recorrer lista de elementos construibles
  (:Pressed
    (Variables|Default|SetBuildableIndex (Math|Integer|Clamp(Integer) (- (Variables|Default|GetBuildableIndex) 1) 0 (- (Utilities|Array|Length (Variables|Default|GetDT_Buildables)) 1)))
    ;[0.15 0.15 0.15 0.5] Hacemos que se actualice el mesh en el preview mode
    (bind _previewmesh (Variables|Default|GetPreviewMesh)
      (:then
        (Components|StaticMesh|SetStaticMesh _previewmesh 0)
        (Variables|Default|SetPreviewMesh 0)
        (CallFunction|ResetBuildMode))
      (:else))))