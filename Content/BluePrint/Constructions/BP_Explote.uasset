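; BP_Explote is a construction actor that works as a one-shot explosive against enemies.
; Each Tick runs the parent logic, then calls Explote as soon as EnemiesList holds any entry.
; Explote deals heavy fixed damage to every listed enemy, then destroys the actor.
; Nothing in this graph fills EnemiesList.
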(event Custom|Explote
  (for _array_element (Variables|Default|GetEnemiesList)
    (Default|TakeDamage _array_element 1e+03))
  (CallFunction|Destroy))

(event Custom|destroy
  (Actor|DestroyActor))

(event EventBeginPlay
  (|CallParentFunction) ; This node is disabled and will not be called.\nDrag off pins to build functionality.
)

(event Collision|EventActorBeginOverlap
  (params (OtherActor :type Actor%20Object%20Reference))
  (|CallParentFunction OtherActor) ; This node is disabled and will not be called.\nDrag off pins to build functionality.
)

(event EventTick
  (params (DeltaSeconds :type Float%20%28single-precision%29))
  (|CallParentFunction DeltaSeconds)
  (if (not (Utilities|Array|IsEmpty (Variables|Default|GetEnemiesList)))
    (CallFunction|Explote)))

(fn ConstructionScript
  (|CallParentFunction))