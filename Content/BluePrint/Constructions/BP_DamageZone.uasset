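; Damage zone Blueprint that hurts every enemy held in its EnemiesList.
; Tick calls the Damage event while the list is not empty, which applies a fixed TakeDamage to each entry when CanDamage is true.
; Damage lands per frame without delta-time scaling, so its rate follows frame rate.
; The graphs shown neither fill the list nor toggle CanDamage.
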(event Custom|Damage
  (if (Variables|Default|GetcanDamage)
    (for _array_element (Variables|Default|GetEnemiesList)
      (Default|TakeDamage _array_element 1.0))))

(event EventBeginPlay
  (|CallParentFunction) ; This node is disabled and will not be called.\nDrag off pins to build functionality.
)

(event Collision|EventActorBeginOverlap
  (params (OtherActor :type Actor%20Object%20Reference))
  (|CallParentFunction OtherActor) ; This node is disabled and will not be called.\nDrag off pins to build functionality.
)

(event EventTick
  (params (DeltaSeconds :type Float%20%28single-precision%29))
  (|CallParentFunction DeltaSeconds)
  (if (not (Utilities|Array|IsEmpty (Variables|Default|GetEnemiesList)))
    (CallFunction|Damage)))

(fn ConstructionScript
  (|CallParentFunction))