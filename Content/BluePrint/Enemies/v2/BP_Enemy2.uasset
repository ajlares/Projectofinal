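; BP_Enemy2 is an enemy pawn that patrols a looping waypoint route, advancing whenever an AI MoveTo succeeds.
; MovePonts supplies the route and restarts movement, which also starts on BeginPlay; a failed move only prints.
; TakeDamage applies half the incoming damage to clamped life and destroys the actor at zero.
; SlowEnemie briefly lowers walk speed, while a ChasePlayer event targeting the player has no wired caller here.
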(event Custom|ChasePlayer
  (AI|AIMoveTo self "0, 0, 0" (Game|GetPlayerCharacter 0) 5.0 false))

(event Custom|follow%20Waypoint
  (Development|PrintString "StartMovement")
  (AI|AIMoveTo self "0, 0, 0" (Utilities|Array|Get(acopy) (Variables|Default|Getwaypoints) (Variables|Default|GetCharacterWaypoint)) 5.0 false
    (:OnSuccess
      (Development|PrintString "sucess move")
      (Math|Integer|IncrementInt (Variables|Default|GetCharacterWaypoint)
        (:%20%20
          (if (>= (Variables|Default|GetCharacterWaypoint) (Utilities|Array|Length (Variables|Default|Getwaypoints)))
            (Variables|Default|SetCharacterWaypoint 0))
          (CallFunction|FollowWaypoint))))
    (:OnFail
      (Development|PrintString "faile move"))))

(event EventBeginPlay
  (bind _output_get (Variables|Default|SetmaxLife 5e+02))
  (Variables|Default|Setlife _output_get)
  (CallFunction|FollowWaypoint))

(event EventMovePonts
  (params (movepoints :type Array%20of%20BP%20Waypoint%20Object%20References))
  (Variables|Default|Setwaypoints movepoints)
  (Development|PrintString "debug")
  (CallFunction|FollowWaypoint))

(event EventTakeDamage
  (params (DamageAmoumt :type Float%20%28double-precision%29))
  (bind _output_get (Variables|Default|Setlife (Math|Float|Clamp(Float) (- (Variables|Default|Getlife) (/ DamageAmoumt 2.0)) 0.0 (Variables|Default|GetmaxLife))))
  (if (<= _output_get 0.0)
    (Actor|DestroyActor)))

(event EventSlowEnemie
  (Variables|/Script/Engine.CharacterMovementComponent|SetMaxWalkSpeed (Variables|Character|GetCharacterMovement) 5e+01)
  (Utilities|FlowControl|Delay 2.0)
  (Variables|/Script/Engine.CharacterMovementComponent|SetMaxWalkSpeed (Variables|Character|GetCharacterMovement) 1e+02))

(fn ConstructionScript)