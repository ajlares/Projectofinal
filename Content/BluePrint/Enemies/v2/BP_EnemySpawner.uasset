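; BP_EnemySpawner is an enemy spawner actor that creates a single random enemy when play begins.
; On BeginPlay it picks a random class from its enemy list and spawns it at the spawner's own transform.
; It then hands its waypoint list to the spawned enemy through MovePonts, presumably setting the enemy's patrol or movement path.
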(event Custom|cretae%20Enemie
  (bind _enemieslist (Variables|Default|GetENemiesList))
  (bind _returnvalue (Game|SpawnActorfromClass (Utilities|Array|Get(acopy) _enemieslist (Math|Random|RandomInteger (Utilities|Array|Length _enemieslist))) (Transformation|GetActorTransform self) "Undefined" "MultiplyWithRoot" 0 0))
  (Default|MovePonts _returnvalue (Variables|Default|GetWayPoints)))

(event EventBeginPlay
  (CallFunction|CretaeEnemie))

(event Collision|EventActorBeginOverlap
  (params (OtherActor :type Actor%20Object%20Reference)))

(event EventTick
  (params (DeltaSeconds :type Float%20%28single-precision%29)))

(fn ConstructionScript)