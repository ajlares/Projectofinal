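; BP_Enemy2 is an enemy actor Blueprint that delegates its damage and movement handling to components.
; Its TakeDamage event forwards the damage amount to the BPACEnemyStats component.
; Its MovePonts event, logged as an interface call, passes move points and the static mesh's world location to BPACEnemyMove, with debug prints around the call.
; BeginPlay, overlap and Tick are disabled stubs.
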(event EventBeginPlay
  (|CallParentFunction) ; This node is disabled and will not be called.\nDrag off pins to build functionality.
)

(event Collision|EventActorBeginOverlap
  (params (OtherActor :type Actor%20Object%20Reference))
  (|CallParentFunction OtherActor) ; This node is disabled and will not be called.\nDrag off pins to build functionality.
)

(event EventTick
  (params (DeltaSeconds :type Float%20%28single-precision%29))
  (|CallParentFunction DeltaSeconds) ; This node is disabled and will not be called.\nDrag off pins to build functionality.
)

(event EventTakeDamage
  (params (DamageAmoumt :type Float%20%28double-precision%29))
  (Class|BPIEnemyConextion|TakeDamage(Message) (Variables|Default|GetBPAC_EnemyStats) DamageAmoumt))

(event EventMovePonts
  (params (movepoints :type Array%20of%20Actor%20Object%20References))
  (Development|PrintString "Interfaz Call Out")
  (Default|Movepoints (Variables|Default|GetBPAC_EnemyMove) movepoints (Transformation|GetWorldLocation (Variables|Default|GetStaticMesh self)))
  (Development|PrintString "Component Call"))

(fn ConstructionScript
  (|CallParentFunction))