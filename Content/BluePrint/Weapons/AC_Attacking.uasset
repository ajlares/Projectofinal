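; AC_Attacking is a component that plays melee-style attack montages on the owning BP_ThirdPersonCharacter, cached with its mesh at BeginPlay.
; IA_Attack, gated by IsAttacking, plays one of four montages chosen by AttackCount, then increments the count.
; Completion resets only the count; interruption waits on a retriggerable delay, then clears both flag and count.
; Nothing else in this graph clears IsAttacking.
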(event Input|EnhancedActionEvents|EnhancedInputActionIA_Attack
  (params (ActionValue :type Boolean) (ElapsedSeconds :type Float%20%28double-precision%29) (TriggeredSeconds :type Float%20%28double-precision%29) (InputAction :type Input%20Action%20Object%20Reference :default "/Game/ThirdPerson/Input/Actions/IA_Attack.IA_Attack"))
  (if (not (Variables|Default|GetIsAttacking))
    (Variables|Default|SetIsAttacking true)
    (Animation|Montage|PlayMontage (Variables|Default|GetPlayerMesh) (Utilities|Select :Index (Variables|Default|GetAttackCount) :Option%200 "/Game/Anims/Montages/Attack1.Attack1" :Option%201 "/Game/Anims/Montages/Attack2.Attack2" :Option%202 "/Game/Anims/Montages/Attack3.Attack3" :Option%203 "/Game/Anims/Montages/Attack4.Attack4")
      (:then
        (Math|Integer|IncrementInt (Variables|Default|GetAttackCount)))
      (:OnCompleted
        (Variables|Default|SetAttackCount 0 :!label _label))
      (:OnInterrupted
        (Utilities|FlowControl|RetriggerableDelay 2.5)
        (Variables|Default|SetIsAttacking false)
        (goto _label)))))

(event EventBeginPlay
  ;[0.15 0.15 0.15 0.5] Conseguir referencia a BP player
  (bind _asbp_third_person_character (Utilities|Casting|CastToBP_ThirdPersonCharacter (Components|GetOwner)))
  (bind _output_get (Variables|Default|SetBP_Player _asbp_third_person_character))
  (Variables|Default|SetPlayerMesh (Variables|/Script/Engine.Character|GetMesh _output_get)))

(event EventTick
  (params (DeltaSeconds :type Float%20%28single-precision%29)))